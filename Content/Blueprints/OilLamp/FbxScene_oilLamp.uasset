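; Oil lamp pickup actor that the GearVR_Char player collects by walking into its Box trigger.
; On overlap it sets IsOilLampPickedUp on the character, adds to PlayerBattery, then destroys itself and plays a 2D match-strike sound.
; The battery cap tests for above zero instead of above the maximum, so any positive result snaps to full charge.
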(event `self.Box.OnComponentBeginOverlap`
  (params (OverlappedComponent :type "PrimitiveComponent Object Reference") (OtherActor :type "Actor Object Reference") (OtherComp :type "PrimitiveComponent Object Reference") (OtherBodyIndex :type Integer) (bFromSweep :type Boolean) (SweepResult :type "HitResult Structure (by ref)"))
  (`|ExecutionSequence`
    (:`then_0`
      (bind _asgear_vr_char (cast `/Game/Blueprints/GearVR_Char` OtherActor))
      (set `/Game/Blueprints/GearVR_Char.IsOilLampPickedUp` true _asgear_vr_char))
    (:`then_1`
      (bind _asgear_vr_char_2 (cast `/Game/Blueprints/GearVR_Char` OtherActor))
      (bind _output_get (set `/Game/Blueprints/GearVR_Char.playerBattery` (+ (`/Game/Blueprints/GearVR_Char.playerBattery` _asgear_vr_char_2) 100) _asgear_vr_char_2))
      (if (> _output_get 0)
        (set `/Game/Blueprints/GearVR_Char.playerBattery` 100 _asgear_vr_char_2))
      (`self.K2_DestroyActor`)
      (`GameplayStatics.PlaySound2D` "/Game/Sounds/MatchStrike.MatchStrike"))))

(fn `UserConstructionScript`)