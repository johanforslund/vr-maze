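; Battery pickup actor for a GearVR character that refills the player's battery on overlap, provided the oil lamp has been picked up.
; Each tick, its point light brightens while it is the character's traced actor and dims otherwise.
; The box overlap adds charge, then sets the battery to 100 whenever the result is above zero, so it normally fills completely.
; The actor then destroys itself and plays a match-strike sound.
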(event `self.ReceiveTick`
  (params (DeltaSeconds :type "Float (single-precision)"))
  (bind _asgear_vr_char (cast `/Game/Blueprints/GearVR_Char` (`GameplayStatics.GetPlayerCharacter` 0)))
  (if (== self (`/Game/Blueprints/GearVR_Char.TracedActor` _asgear_vr_char))
    (`LightComponent.SetIntensity` (`self.PointLight`) 5000.0)
    (else
      (`LightComponent.SetIntensity` (`self.PointLight`) 2500.0))))

(event `self.Box.OnComponentBeginOverlap`
  (params (OverlappedComponent :type "PrimitiveComponent Object Reference") (OtherActor :type "Actor Object Reference") (OtherComp :type "PrimitiveComponent Object Reference") (OtherBodyIndex :type Integer) (bFromSweep :type Boolean) (SweepResult :type "HitResult Structure (by ref)"))
  (bind _asgear_vr_char (cast `/Game/Blueprints/GearVR_Char` OtherActor))
  (if (`/Game/Blueprints/GearVR_Char.IsOilLampPickedUp` _asgear_vr_char)
    (bind _asgear_vr_char_2 (cast `/Game/Blueprints/GearVR_Char` OtherActor))
    (bind _output_get (set `/Game/Blueprints/GearVR_Char.playerBattery` (+ (`/Game/Blueprints/GearVR_Char.playerBattery` _asgear_vr_char_2) 25) _asgear_vr_char_2))
    (if (> _output_get 0)
      (set `/Game/Blueprints/GearVR_Char.playerBattery` 100 _asgear_vr_char_2))
    (`self.K2_DestroyActor`)
    (`GameplayStatics.PlaySound2D` "/Game/Sounds/MatchStrike.MatchStrike")))

(fn `UserConstructionScript`)